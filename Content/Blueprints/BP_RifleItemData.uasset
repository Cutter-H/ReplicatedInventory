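; BP_RifleItemData is the item data Blueprint for the rifle, supplying the text shown for it in a grid display, likely an inventory.
; It overrides GetGridDisplayText to cast its owner to BP_Pickup_Rifle and return current and maximum ammo as a "current/max" string.
; If the owner is not a rifle pickup, it falls back to the parent implementation.
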(fn `GetGridDisplayText`
  (returns (ReturnValue :type Text))
  (bind _asbp_pickup_rifle (cast `/ReplicatedInventory/Demo/FirstPersonTemplate/FirstPerson/Blueprints/BP_Pickup_Rifle` (`self.GetOwner`))
    (:`then`
      (return (`KismetTextLibrary.Conv_StringToText` (`KismetStringLibrary.Concat_StrStr` (`KismetStringLibrary.Conv_IntToString` (`/ReplicatedInventory/Demo/FirstPersonTemplate/FirstPerson/Blueprints/BP_Pickup_Rifle.CurrentAmmo` _asbp_pickup_rifle)) " / " (`KismetStringLibrary.Conv_IntToString` (`/ReplicatedInventory/Demo/FirstPersonTemplate/FirstPerson/Blueprints/BP_Pickup_Rifle.MaxAmmo` _asbp_pickup_rifle))))))
    (:`CastFailed`
      (return (`parent.GetGridDisplayText`)))))