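; Base item pickup actor that adds its item to an overlapping actor's inventory.
; On server-side sphere overlap, it looks for an InventoryComponent on that actor and passes in the item data from GetItemDataComp, which is empty here.
; On success, ReplicatePickup hides the visuals, plays a pickup sound and disables sphere collision without destroying the actor; failure only prints a message.
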(event `self.Sphere.OnComponentBeginOverlap`
  (params (OverlappedComponent :type "PrimitiveComponent Object Reference") (OtherActor :type "Actor Object Reference") (OtherComp :type "PrimitiveComponent Object Reference") (OtherBodyIndex :type Integer) (bFromSweep :type Boolean) (SweepResult :type "HitResult Structure (by ref)"))
  (bind _returnvalue (`self.GetComponentByClass` OtherActor "/Script/ReplicatedInventory.InventoryComponent"))
  (`/Engine/EditorBlueprintResources/ActorMacros.Switch Has Authority` ; Only on the server so the pickup \nis replicated correctly.
    (:`Authority`
      (`/Engine/EditorBlueprintResources/StandardMacros.IsValid` _returnvalue ; Does the actor have an Inventory?\n\nFurther detection will be required if the inventory is on the player state or other class.
        (:`Is Valid`
          (bind _returnvalue_2 (`InventoryComponent.AddItemComponentToInventory` _returnvalue (`self.GetItemDataComp`) -1))
          (if (< _returnvalue_2 0)
            (`KismetSystemLibrary.PrintString` "Failed to add")
            (else
              (`self.ReplicatePickup`))))))))

(event `ReplicatePickup`
  (`SceneComponent.SetVisibility` (`self.DefaultSceneRoot`) false true)
  (`GameplayStatics.PlaySoundAtLocation` "/ReplicatedInventory/Demo/EngineAssets/Object_PickUp.Object_PickUp" (`self.K2_GetActorLocation`) (struct) 1.0 1.0 0.0 null null null null)
  (`PrimitiveComponent.SetCollisionEnabled` (`self.Sphere`) "NoCollision"))

(fn `GetItemDataComp`
  (returns (ReturnValue :type "ItemDataComponent Object Reference"))
  (return null))

(fn `UserConstructionScript`)