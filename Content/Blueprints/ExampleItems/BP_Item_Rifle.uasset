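; Example rifle item for the inventory system that can be equipped in first person and fired.
; On equip it attaches to the character's GripPoint through the server, multicasts visibility, sets the anim blueprint's rifle flag, enables input and adds an ammo widget.
; Pressing 1 spends a round, refreshes the item data's grid text and the widget, then plays the shoot montage and sound, with no projectile or trace.
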(event `ReplicateEquippedVisibility`
  (`SceneComponent.SetVisibility` (`self.SkeletalMesh`) true false)
  (bind _asbp_inventory_character (cast `/ReplicatedInventory/Demo/FirstPersonTemplate/FirstPerson/Blueprints/BP_InventoryCharacter` (`self.GetParentActor`)))
  (bind _asfirst_person_abp (cast `/ReplicatedInventory/Demo/FirstPersonTemplate/FirstPersonArms/Animations/FirstPerson_ABP` (`SkeletalMeshComponent.GetAnimInstance` (`/ReplicatedInventory/Demo/FirstPersonTemplate/FirstPerson/Blueprints/BP_InventoryCharacter.FirstPersonMesh` _asbp_inventory_character))))
  (set `/ReplicatedInventory/Demo/FirstPersonTemplate/FirstPersonArms/Animations/FirstPerson_ABP.HasRifle` true _asfirst_person_abp))

(event `SnapGunToCharacterBone`
  (params (meshComponent :type "SkeletalMeshComponent Object Reference") (boneName :type Name))
  (`self.K2_AttachToComponent` meshComponent boneName "SnapToTarget" "SnapToTarget" "KeepRelative")
  (`self.ReplicateEquippedVisibility`))

(event `EquipWeapon`
  (params (EquippingActor :type "Actor Object Reference"))
  (bind _returnvalue (`GameplayStatics.GetPlayerController` 0))
  (bind _asbp_inventory_character (cast `/ReplicatedInventory/Demo/FirstPersonTemplate/FirstPerson/Blueprints/BP_InventoryCharacter` EquippingActor))
  (`|ExecutionSequence`
    (:`then_0`
      (`/Engine/EditorBlueprintResources/ActorMacros.Switch Has Authority`
        (:`Authority`
          (bind _firstpersonmesh (`/ReplicatedInventory/Demo/FirstPersonTemplate/FirstPerson/Blueprints/BP_InventoryCharacter.FirstPersonMesh` _asbp_inventory_character))
          (`self.K2_AttachToComponent` _firstpersonmesh "GripPoint" "SnapToTarget" "SnapToTarget" "KeepRelative")
          (`self.ReplicateEquippedVisibility`))
        (:`Remote`
          (`self.SnapGunToCharacterBone` _firstpersonmesh "GripPoint")))
      (bind _asbp_inventory_character_2 (cast `/ReplicatedInventory/Demo/FirstPersonTemplate/FirstPerson/Blueprints/BP_InventoryCharacter` (`self.GetOwner`)))
      (bind _asfirst_person_abp (cast `/ReplicatedInventory/Demo/FirstPersonTemplate/FirstPersonArms/Animations/FirstPerson_ABP` (`SkeletalMeshComponent.GetAnimInstance` (`/ReplicatedInventory/Demo/FirstPersonTemplate/FirstPerson/Blueprints/BP_InventoryCharacter.FirstPersonMesh` _asbp_inventory_character_2))))
      (set `/ReplicatedInventory/Demo/FirstPersonTemplate/FirstPersonArms/Animations/FirstPerson_ABP.HasRifle` true _asfirst_person_abp))
    (:`then_1`
      (`self.EnableInput` _returnvalue)
      (bind _returnvalue_2 (`|CreateWidget` "/ReplicatedInventory/Blueprints/UI/WBP_EquippedFirearmAmmo.WBP_EquippedFirearmAmmo_C" _returnvalue self))
      (bind _output_get (set `self.Widget` _returnvalue_2))
      (`UserWidget.AddToPlayerScreen` _output_get 0))))

(event `Key|One`
  (params (Key :type "Key Structure"))
  (bind _bp_rifleitemdata (`self.BP_RifleItemData`))
  (:`Pressed`
    (if (> (`self.CurrentAmmo`) 0)
      (`/Engine/EditorBlueprintResources/StandardMacros.DecrementInt` (`self.CurrentAmmo`)
        (:`  `
          (`ItemDataComponent.OnGridTextChange` _bp_rifleitemdata (`ItemDataComponent.GetGridDisplayText` _bp_rifleitemdata))
          (bind _widget (`self.Widget`)
            (:`then`
              (`/ReplicatedInventory/Blueprints/UI/WBP_EquippedFirearmAmmo.UpdateText` _widget)
              (bind _asbp_inventory_character (cast `/ReplicatedInventory/Demo/FirstPersonTemplate/FirstPerson/Blueprints/BP_InventoryCharacter` (`self.GetOwner`)))
              (`|PlayMontage` (`/ReplicatedInventory/Demo/FirstPersonTemplate/FirstPerson/Blueprints/BP_InventoryCharacter.FirstPersonMesh` _asbp_inventory_character) "/ReplicatedInventory/Demo/FirstPersonTemplate/FirstPersonArms/Animations/FP_Rifle_Shoot_Montage.FP_Rifle_Shoot_Montage"
                (:`then`
                  (`GameplayStatics.PlaySound2D` "/ReplicatedInventory/Demo/FirstPersonTemplate/FPGun/Audio/FirstPersonTemplateWeaponFire02.FirstPersonTemplateWeaponFire02" 1.0 1.0 0.0 null null))))
            (:`else`)))))))

(fn `GetItemDataComp`
  (returns (ReturnValue :type "ItemDataComponent Object Reference"))
  (return (`self.BP_RifleItemData`)))

(fn `UserConstructionScript`)