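; BP_RifleItemData is the item data for the example rifle item, supplying the rifle's ammo readout as its grid display text.
; It overrides GetGridDisplayText, casting its owner to BP_Item_Rifle and formatting the result as current ammo over max ammo.
; When the owner is not a rifle, it falls back to the parent's text.
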(fn `GetGridDisplayText`
  (returns (ReturnValue :type Text))
  (bind _asbp_item_rifle (cast `/ReplicatedInventory/Blueprints/ExampleItems/BP_Item_Rifle` (`self.GetOwner`))
    (:`then`
      (return (`KismetTextLibrary.Conv_StringToText` (`KismetStringLibrary.Concat_StrStr` (`KismetStringLibrary.Conv_IntToString` (`/ReplicatedInventory/Blueprints/ExampleItems/BP_Item_Rifle.CurrentAmmo` _asbp_item_rifle)) " / " (`KismetStringLibrary.Conv_IntToString` (`/ReplicatedInventory/Blueprints/ExampleItems/BP_Item_Rifle.MaxAmmo` _asbp_item_rifle))))))
    (:`CastFailed`
      (return (`parent.GetGridDisplayText`)))))